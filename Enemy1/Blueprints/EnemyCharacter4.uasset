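; EnemyCharacter4 is an enemy character that chases the explorer player when its PawnSensing component sees them, using AI MoveTo.
; TakeDamage subtracts from HP and pushes the value to the avatar progress bar on player 0's HUD.
; Death disables input from player 0's controller and plays a death animation, but nothing here calls it.
; MoveForward and MoveRight axis handlers also add movement along fixed world axes.
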(event `self.PawnSensing.OnSeePawn`
  (params (Pawn :type "Pawn Object Reference"))
  (bind _asexplorer_third_person_character (cast `/Game/ThirdPersonBP/Blueprints/ExplorerThirdPersonCharacter` Pawn))
  (`|AIMoveTo` self (0.0 0.0 0.0) _asexplorer_third_person_character))

(event `InputAxis|MoveForward` :overrideparent false
  (params (AxisValue :type "Float (single-precision)"))
  (`self.AddMovementInput` (`KismetMathLibrary.GetForwardVector` (struct)) AxisValue))

(event `InputAxis|MoveRight` :overrideparent false
  (params (AxisValue :type "Float (single-precision)"))
  (`self.AddMovementInput` (`KismetMathLibrary.GetRightVector` (struct)) AxisValue))

(fn `Death`
  (`self.DisableInput` (`GameplayStatics.GetPlayerController` 0))
  (`SkeletalMeshComponent.PlayAnimation` (`self.Mesh`) "/Game/AnimStarterPack/Death_2.Death_2" false))

(fn `TakeDamage`
  (params (Damage :type Integer))
  (set `self.HP` (- (`self.HP`) Damage))
  (`/Game/UI/UI_Avatar._UpdateProgress` (`/Game/UI/UI_GameHUD.UI_Avatar` (`/Game/Ruins/Character/ThirdPersonBP/Blueprints/APlayerController.GameHUD` (cast `/Game/Ruins/Character/ThirdPersonBP/Blueprints/APlayerController` (`GameplayStatics.GetPlayerController` 0) :!pure true))) (`self.HP`) (`self.MaxHP`) true))

(fn `UserConstructionScript`)